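; Character Blueprint for the Blaster character that handles the sniper scope overlay and its zoom sounds.
; The ShowSniperScopeWidget event creates WBP_SniperScope on first use, adds it to the viewport and keeps the reference for later calls.
; Its ShowScope flag plays the widget's zoom animation forward or in reverse, paired with a 2D zoom-in or zoom-out cue.
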(event `self.ShowSniperScopeWidget`
  (params (bShowScope :type Boolean))
  (`self.SniperScoreWidget`
    (:`then`
      _)
    (:`else`
      (bind _returnvalue (`|CreateWidget` "/Game/Blueprints/HUD/WBP_SniperScope.WBP_SniperScope_C"))
      (bind _output_get (set `self.SniperScoreWidget` _returnvalue))
      (`UserWidget.AddToViewport` _output_get 0)))
  (bind _sniperscorewidget (`self.SniperScoreWidget`)
    (:`then`
      (if bShowScope
        (bind _scopezoominanim (`/Game/Blueprints/HUD/WBP_SniperScope.ScopeZoomInAnim` _sniperscorewidget))
        (`UserWidget.PlayAnimationForward` (`self.SniperScoreWidget`) _scopezoominanim 1.0 false)
        (`GameplayStatics.PlaySound2D` "/Game/Assets/MilitaryWeapSilver/Sound/SniperRifle/Cues/SniperRifle_ZoomIn_Cue.SniperRifle_ZoomIn_Cue" 1.0 1.0 0.0 null null)
        (else
          (`UserWidget.PlayAnimationReverse` (`self.SniperScoreWidget`) _scopezoominanim 1.0 false)
          (`GameplayStatics.PlaySound2D` "/Game/Assets/MilitaryWeapSilver/Sound/SniperRifle/Cues/SniperRifle_ZoomOut_Cue.SniperRifle_ZoomOut_Cue" 1.0 1.0 0.0 null null))))
    (:`else`)))

(fn `UserConstructionScript`)